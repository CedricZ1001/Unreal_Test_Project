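; Character component that adds spreading blood soak spots to a skeletal mesh where it is hit.
; Initialize caches every bone's reference-pose transform and creates dynamic materials unless another wound component exists on the owner.
; TakeHit maps the world hit into reference-pose space, so spots follow the animated body, up to a spot limit.
; Tick grows each radius to its maximum, packing location and radius into indexed material vector parameters, then switches itself off.
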(event `self.ReceiveBeginPlay`)

(event `Initialize`
  (params (SkeletalMesh :type "SkeletalMeshComponent Object Reference"))
  (bind _skeletalmesh (`self.GetMesh`))
  (bind _returnvalue (`self.GetOwner`))
  (bind _skeletalmesh_2 (`self.GetMesh`))
  (bind _output_get (set `self.MeshReference` SkeletalMesh))
  (`/Engine/EditorBlueprintResources/StandardMacros.IsValid` _output_get
    (:`Is Valid`
      _)
    (:`Is Not Valid`
      (`KismetSystemLibrary.PrintString` "BloodSoakingComponent: Invalid SkeletalMesh component" false true (struct :`R` 1.0 :`G` 0.144209 :`A` 1.0))
      (bind _ascharacter (cast `Character` (`self.GetOwner`)))
      (set `self.MeshReference` (`Character.Mesh` _ascharacter))))
  (`|ExecutionSequence`
    (:`then_0`
      ;[0.1 0.5 1] Configure components
      (`PrimitiveComponent.SetCollisionObjectType` _skeletalmesh_2 "ECC_WorldDynamic")
      (`PrimitiveComponent.SetCollisionEnabled` _skeletalmesh_2 "QueryOnly")
      (`PrimitiveComponent.SetCollisionResponseToChannel` _skeletalmesh_2 "ECC_Visibility" "ECR_Block"))
    (:`then_1`
      ;[1 0.3 0] Store all bones Reference Pose Transforms so we don't need to calculate this every time
      (`self.CalculateRefTransforms`))
    (:`then_2`
      ;[0.1 1 0.1 0.5] If there's no other wound component in this character, store the materials here
      (if (not (or (> (`KismetArrayLibrary.Array_Length` (`Actor.K2_GetComponentsByClass` _returnvalue "/Game/CharacterWoundSystem/Blueprint/Components/WoundComponent.WoundComponent_C")) 0) (> (`KismetArrayLibrary.Array_Length` (`Actor.K2_GetComponentsByClass` _returnvalue "/Game/CharacterWoundSystem/Blueprint/Components/ProjectedWoundComponent.ProjectedWoundComponent_C")) 0)))
        (for (_ _array_index) (`MeshComponent.GetMaterials` _skeletalmesh)
          (`PrimitiveComponent.CreateDynamicMaterialInstance` _skeletalmesh _array_index null "None"))))))

(event `self.ReceiveTick`
  (params (DeltaSeconds :type "Float (single-precision)"))
  ;[0.2 0.2 0.2 0.2] Tick for updating the radiuses
  (if (not (`self.DoneUpdating`))
    (`self.UpdateValues` DeltaSeconds)))

(event `LateInitialize`
  ;[0.2 0.2 0.2 0.2] To make things a bit easier if you forget to initiliaze this component then do it manually
  (`/Engine/EditorBlueprintResources/StandardMacros.IsValid` (`self.GetMesh`)
    (:`Is Not Valid`
      (bind _ascharacter (cast `Character` (`self.GetOwner`)))
      (`self.Initialize` (`Character.Mesh` _ascharacter)))))

(event `TakeHit`
  (params (Location :type "Vector Structure") (BoneName :type Name) (Radius :type "Float (double-precision)" :default 15.0) (SpreadSpeed :type "Float (double-precision)" :default 1.0) (InitialRadius :type "Float (double-precision)"))
  (`self.LateInitialize`)
  (if (< (`KismetArrayLibrary.Array_Length` (`self.Locations`)) (`self.MaxSpots`))
    (`KismetArrayLibrary.Array_Add` (`self.Locations`) (`self.TransformLocationByRefBoneTransform` BoneName Location))
    (`KismetArrayLibrary.Array_Add` (`self.MaxRadiuses`) Radius)
    (`KismetArrayLibrary.Array_Add` (`self.SpreadVelocities`) SpreadSpeed)
    (`KismetArrayLibrary.Array_Add` (`self.Radiuses`) InitialRadius)
    (if (< InitialRadius Radius)
      (set `self.DoneUpdating` false)
      (`self.SetComponentTickEnabled` true)
      (else
        (`self.UpdateMaterialParameters`)))))

(fn `CalculateRefTransforms`
  (bind _skeletalmesh (`self.GetMesh`))
  (for _index (range (+ (`SkinnedMeshComponent.GetNumBones` _skeletalmesh) 1))
    (bind _meshlocalspacetransform (`self.GetRefPoseBoneTransform` _skeletalmesh (`SkinnedMeshComponent.GetBoneName` _skeletalmesh _index)))
    (`KismetArrayLibrary.Array_Add` (`self.RefPoseLocalBoneTransforms`) _meshlocalspacetransform)))

(fn `GetMesh`
  (returns (SkeletalMesh :type "SkeletalMeshComponent Object Reference"))
  (return (`self.MeshReference`)))

(fn `GetRefPoseBoneTransform`
  (params (SkeletalMesh :type "SkeletalMeshComponent Object Reference") (BoneName :type Name))
  (returns (MeshLocalSpaceTransform :type "Transform Structure"))
  (locals (BoneTransform :type "Transform Structure"))
  (bind _returnvalue (`SkinnedMeshComponent.GetParentBone` SkeletalMesh BoneName))
  (bind _returnvalue_2 (`KismetMathLibrary.InvertTransform` (`SkinnedMeshComponent.GetDeltaTransformFromRefPose` SkeletalMesh BoneName "None")))
  (if (!= _returnvalue "None")
    (bind _meshlocalspacetransform (`self.GetRefPoseBoneTransform` SkeletalMesh _returnvalue))
    (set `local.BoneTransform` (`KismetMathLibrary.ComposeTransforms` (`KismetMathLibrary.ComposeTransforms` _returnvalue_2 (`SceneComponent.GetSocketTransform` SkeletalMesh BoneName "RTS_ParentBoneSpace")) _meshlocalspacetransform))
    (else
      (set `local.BoneTransform` (`KismetMathLibrary.ComposeTransforms` _returnvalue_2 (`SceneComponent.GetSocketTransform` SkeletalMesh BoneName "RTS_World")))))
  (return (`local.BoneTransform`)))

(fn `TransformDirectionByRefBoneTransform`
  (params (BoneName :type Name) (WorldDirection :type "Vector Structure"))
  (returns (MeshLocalSpaceDirection :type "Vector Structure"))
  (bind _skeletalmesh (`self.GetMesh`))
  (bind _returnvalue (`SkinnedMeshComponent.GetBoneIndex` _skeletalmesh BoneName))
  (`self.LateInitialize`)
  (if (!= _returnvalue -1)
    (return (`KismetMathLibrary.TransformDirection` (`KismetMathLibrary.ComposeTransforms` (`KismetMathLibrary.InvertTransform` (`SceneComponent.GetSocketTransform` _skeletalmesh BoneName "RTS_Component")) (`|GetArrayItem` (`self.RefPoseLocalBoneTransforms`) _returnvalue)) (`KismetMathLibrary.InverseTransformDirection` (`SceneComponent.K2_GetComponentToWorld` _skeletalmesh) WorldDirection)))
    (else
      (`self.WarningBoneName` BoneName))))

(fn `TransformLocationByRefBoneTransform`
  (params (BoneName :type Name) (WorldLocation :type "Vector Structure"))
  (returns (MeshLocalSpaceLocation :type "Vector Structure"))
  (bind _meshreference (`self.MeshReference`))
  (bind _returnvalue (`SkinnedMeshComponent.GetBoneIndex` _meshreference BoneName))
  (`self.LateInitialize`)
  (if (!= _returnvalue -1)
    (return (`KismetMathLibrary.TransformLocation` (`KismetMathLibrary.ComposeTransforms` (`KismetMathLibrary.InvertTransform` (`SceneComponent.GetSocketTransform` _meshreference BoneName "RTS_Component")) (`|GetArrayItem` (`self.RefPoseLocalBoneTransforms`) _returnvalue)) (`KismetMathLibrary.InverseTransformLocation` (`SceneComponent.K2_GetComponentToWorld` _meshreference) WorldLocation)))
    (else
      (`self.WarningBoneName` BoneName))))

(fn `UpdateMaterialArrayParameters`
  (params (Materials :type "Array of MaterialInterface Object Reference"))
  (for _array_element Materials
    (bind _asmaterial_instance_dynamic (cast `MaterialInstanceDynamic` _array_element))
    (for (_array_element_2 _array_index) (`self.Locations`)
      (`MaterialInstanceDynamic.SetVectorParameterValue` _asmaterial_instance_dynamic (`KismetStringLibrary.Conv_StringToName` (`KismetStringLibrary.Concat_StrStr` "SLocation_" (`KismetStringLibrary.Conv_IntToString` _array_index))) (make `LinearColor` (.x _array_element_2) (.y _array_element_2) (.z _array_element_2) (`|GetArrayItem` (`self.Radiuses`) _array_index))))))

(fn `UpdateMaterialParameters`
  (`self.UpdateMaterialArrayParameters` (`MeshComponent.GetMaterials` (`self.GetMesh`))))

(fn `UpdateValues`
  (params (DeltaSeconds :type "Float (double-precision)"))
  (locals (StillUpdating :type Boolean))
  (bind _radiuses (`self.Radiuses`))
  (`|ExecutionSequence`
    (:`then_0`
      ;[0.2 0.2 0.2 0.2] Increase the radiuses over time
      (for (_array_element _array_index) _radiuses
        (bind _output (`|GetArrayItem` (`self.MaxRadiuses`) _array_index))
        (bind _returnvalue (`KismetMathLibrary.FMin` (+ _array_element (* (`|GetArrayItem` (`self.SpreadVelocities`) _array_index) DeltaSeconds _output)) _output))
        (`KismetArrayLibrary.Array_Set` _radiuses _array_index _returnvalue)
        (if (< _returnvalue _output)
          (set `local.StillUpdating` true)))
      (bind _output_get (set `self.DoneUpdating` (not (`local.StillUpdating`))))
      (if _output_get
        (`self.SetComponentTickEnabled` false)))
    (:`then_1`
      (`self.UpdateMaterialParameters`))))

(fn `WarningBoneName`
  (params (BoneName :type Name))
  (`KismetSystemLibrary.PrintString` (`KismetStringLibrary.Concat_StrStr` "Warning: Wound System Invalid Bone Name : " (`KismetStringLibrary.Conv_NameToString` BoneName)) true true (struct :`R` 1.0 :`G` 0.797118 :`A` 1.0)))