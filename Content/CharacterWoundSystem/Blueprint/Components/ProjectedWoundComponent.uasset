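; Component that adds projected wounds to a skeletal mesh through material parameters, up to MaxWounds hits.
; Initialize makes the mesh block Visibility queries, caches recursively computed reference-pose bone transforms, and creates dynamic materials with wound textures.
; TakeHit converts world hit location and direction into reference-pose space via the hit bone.
; It writes them to indexed material vectors, packing rotation into direction alpha, while one WoundRadius scalar is shared by all wounds.
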(event `self.ReceiveBeginPlay`)

(event `Initialize`
  (params (SkeletalMesh :type "SkeletalMeshComponent Object Reference"))
  (bind _skeletalmesh (`self.GetMesh`))
  (set `self.MeshReference` SkeletalMesh)
  (`|ExecutionSequence`
    (:`then_0`
      ;[0.1 0.5 1] Configure components
      (`PrimitiveComponent.SetCollisionObjectType` _skeletalmesh "ECC_WorldDynamic")
      (`PrimitiveComponent.SetCollisionEnabled` _skeletalmesh "QueryOnly")
      (`PrimitiveComponent.SetCollisionResponseToChannel` _skeletalmesh "ECC_Visibility" "ECR_Block"))
    (:`then_1`
      ;[1 0.3 0] Store all bones Reference Pose Transforms so we don't need to calculate this every time
      (`self.CalculateRefTransforms`))
    (:`then_2`
      ;[0.1 1 0.1 0.5] Create the dynamic materials
      (for (_ _array_index) (`MeshComponent.GetMaterials` SkeletalMesh)
        (bind _returnvalue (`PrimitiveComponent.CreateDynamicMaterialInstance` SkeletalMesh _array_index null "None"))
        (`MaterialInstanceDynamic.SetTextureParameterValue` _returnvalue "WoundTexture" (`self.WoundTexture`))
        (`MaterialInstanceDynamic.SetTextureParameterValue` _returnvalue "WoundNormalTexture" (`self.WoundNormalTexture`))))))

(event `TakeHit`
  (params (Location :type "Vector Structure") (Direction :type "Vector Structure") (WoundRadius :type "Float (double-precision)" :default 5.0) (Rotation :type "Float (double-precision)" :default 15.0) (BoneName :type Name))
  (bind _meshlocalspacelocation (`self.TransformLocationByRefBoneTransform` BoneName Location))
  (bind _meshlocalspacedirection (`self.TransformDirectionByRefBoneTransform` BoneName Direction))
  (bind _returnvalue (`KismetStringLibrary.Conv_IntToString` (- (`KismetArrayLibrary.Array_Length` (`self.Locations`)) 1)))
  (if (< (`KismetArrayLibrary.Array_Length` (`self.Locations`)) (`self.MaxWounds`))
    (`KismetArrayLibrary.Array_Add` (`self.Locations`) _meshlocalspacelocation)
    (`KismetArrayLibrary.Array_Add` (`self.Directions`) _meshlocalspacedirection)
    (`KismetArrayLibrary.Array_Add` (`self.Rotations`) Rotation)
    ;[0 0.2 1 0.2] Send parameters to the materials
    (for _array_element (`MeshComponent.GetMaterials` (`self.GetMesh`))
      (bind _asmaterial_instance_dynamic (cast `MaterialInstanceDynamic` _array_element))
      (`MaterialInstanceDynamic.SetVectorParameterValue` _asmaterial_instance_dynamic (`KismetStringLibrary.Conv_StringToName` (`KismetStringLibrary.Concat_StrStr` "HitLocation_" _returnvalue)) (make `LinearColor` (.x _meshlocalspacelocation) (.y _meshlocalspacelocation) (.z _meshlocalspacelocation) 1.0))
      (`MaterialInstanceDynamic.SetVectorParameterValue` _asmaterial_instance_dynamic (`KismetStringLibrary.Conv_StringToName` (`KismetStringLibrary.Concat_StrStr` "HitDirection_" _returnvalue)) (make `LinearColor` (.x _meshlocalspacedirection) (.y _meshlocalspacedirection) (.z _meshlocalspacedirection) Rotation))
      (`MaterialInstanceDynamic.SetScalarParameterValue` _asmaterial_instance_dynamic "WoundRadius" WoundRadius))))

(fn `CalculateRefTransforms`
  (bind _skeletalmesh (`self.GetMesh`))
  (for _index (range (+ (`SkinnedMeshComponent.GetNumBones` _skeletalmesh) 1))
    (bind _meshlocalspacetransform (`self.GetRefPoseBoneTransform` _skeletalmesh (`SkinnedMeshComponent.GetBoneName` _skeletalmesh _index)))
    (`KismetArrayLibrary.Array_Add` (`self.RefPoseLocalBoneTransforms`) _meshlocalspacetransform)))

(fn `GetMesh`
  (returns (SkeletalMesh :type "SkeletalMeshComponent Object Reference"))
  (return (`self.MeshReference`)))

(fn `GetRefPoseBoneTransform`
  (params (SkeletalMesh :type "SkeletalMeshComponent Object Reference") (BoneName :type Name))
  (returns (MeshLocalSpaceTransform :type "Transform Structure"))
  (locals (BoneTransform :type "Transform Structure"))
  (bind _returnvalue (`SkinnedMeshComponent.GetParentBone` SkeletalMesh BoneName))
  (bind _returnvalue_2 (`KismetMathLibrary.InvertTransform` (`SkinnedMeshComponent.GetDeltaTransformFromRefPose` SkeletalMesh BoneName "None")))
  (if (!= _returnvalue "None")
    (bind _meshlocalspacetransform (`self.GetRefPoseBoneTransform` SkeletalMesh _returnvalue))
    (set `local.BoneTransform` (`KismetMathLibrary.ComposeTransforms` (`KismetMathLibrary.ComposeTransforms` _returnvalue_2 (`SceneComponent.GetSocketTransform` SkeletalMesh BoneName "RTS_ParentBoneSpace")) _meshlocalspacetransform))
    (else
      (set `local.BoneTransform` (`KismetMathLibrary.ComposeTransforms` _returnvalue_2 (`SceneComponent.GetSocketTransform` SkeletalMesh BoneName "RTS_World")))))
  (return (`local.BoneTransform`)))

(fn `TransformDirectionByRefBoneTransform`
  (params (BoneName :type Name) (WorldDirection :type "Vector Structure"))
  (returns (MeshLocalSpaceDirection :type "Vector Structure"))
  (bind _skeletalmesh (`self.GetMesh`))
  (bind _returnvalue (`SkinnedMeshComponent.GetBoneIndex` _skeletalmesh BoneName))
  (if (!= _returnvalue -1)
    (return (`KismetMathLibrary.TransformDirection` (`KismetMathLibrary.ComposeTransforms` (`KismetMathLibrary.InvertTransform` (`SceneComponent.GetSocketTransform` _skeletalmesh BoneName "RTS_Component")) (`|GetArrayItem` (`self.RefPoseLocalBoneTransforms`) _returnvalue)) (`KismetMathLibrary.InverseTransformDirection` (`SceneComponent.K2_GetComponentToWorld` _skeletalmesh) WorldDirection)))
    (else
      (`self.WarningBoneName` BoneName))))

(fn `TransformLocationByRefBoneTransform`
  (params (BoneName :type Name) (WorldLocation :type "Vector Structure"))
  (returns (MeshLocalSpaceLocation :type "Vector Structure"))
  (bind _skeletalmesh (`self.GetMesh`))
  (bind _returnvalue (`SkinnedMeshComponent.GetBoneIndex` _skeletalmesh BoneName))
  (if (!= _returnvalue -1)
    (return (`KismetMathLibrary.TransformLocation` (`KismetMathLibrary.ComposeTransforms` (`KismetMathLibrary.InvertTransform` (`SceneComponent.GetSocketTransform` _skeletalmesh BoneName "RTS_Component")) (`|GetArrayItem` (`self.RefPoseLocalBoneTransforms`) _returnvalue)) (`KismetMathLibrary.InverseTransformLocation` (`SceneComponent.K2_GetComponentToWorld` _skeletalmesh) WorldLocation)))
    (else
      (`self.WarningBoneName` BoneName))))

(fn `WarningBoneName`
  (params (BoneName :type Name))
  (`KismetSystemLibrary.PrintString` (`KismetStringLibrary.Concat_StrStr` "Warning: Wound System Invalid Bone Name : " (`KismetStringLibrary.Conv_NameToString` BoneName)) true true (struct :`R` 1.0 :`G` 0.797118 :`A` 1.0)))