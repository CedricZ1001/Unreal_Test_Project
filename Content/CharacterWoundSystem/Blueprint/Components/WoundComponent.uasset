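; Wound component that paints blood or projected wound textures onto a character's skeletal mesh at hit points.
; Initialize caches reference-pose bone transforms, configures an orthographic SceneCapture and feeds a BloodMask render target to the mesh's materials.
; TakeHit maps hits into reference-pose space, then briefly swaps all mesh materials for a render material to capture the wound into the mask.
; An optional dilation pass hides UV seams.
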(event `self.ReceiveBeginPlay`)

(event `Initialize`
  (params (SkeletalMesh :type "SkeletalMeshComponent Object Reference") (SceneCapture :type "SceneCaptureComponent2D Object Reference"))
  (bind _skeletalmesh (`self.GetMesh`))
  (bind _scenecapturecomponent2d (`self.SceneCaptureComponent2D`))
  (bind _bloodmasksize (`self.BloodMaskSize`))
  (bind _bloodmasksize_2 (`self.BloodMaskSize`))
  (bind _scenecapturecomponent2d_2 (`self.SceneCaptureComponent2D`))
  (`/Engine/EditorBlueprintResources/StandardMacros.IsValid` SkeletalMesh
    (:`Is Valid`
      (`/Engine/EditorBlueprintResources/StandardMacros.IsValid` SceneCapture
        (:`Is Valid`
          (set `self.MeshReference` SkeletalMesh)
          (set `self.SceneCaptureComponent2D` SceneCapture)
          (set `self.BloodMaskInitialized` true)
          (`|ExecutionSequence`
            (:`then_0`
              ;[0.1 0.5 1] Configure components
              (set `SceneCaptureComponent2D.ProjectionType` "Orthographic" _scenecapturecomponent2d_2)
              (set `SceneCaptureComponent2D.OrthoWidth` 1000.0 _scenecapturecomponent2d_2)
              (set `SceneCaptureComponent2D.CompositeMode` "SCCM_Composite" _scenecapturecomponent2d_2)
              (set `SceneCaptureComponent.bCaptureEveryFrame` false _scenecapturecomponent2d_2)
              (set `SceneCaptureComponent.bCaptureOnMovement` false _scenecapturecomponent2d_2)
              (set `SceneCaptureComponent.ShowFlagSettings` (`|MakeArray` (make `EngineShowFlagsSetting` "Skeletal Meshes" true)) _scenecapturecomponent2d_2)
              (`SceneComponent.K2_SetRelativeTransform` _scenecapturecomponent2d_2 (`KismetMathLibrary.MakeTransform` (0.0 0.0 250.0) (struct :`Pitch` -90.0 :`Yaw` 90.0 :`Roll` 180.0)) false false))
            (:`then_1`
              (`PrimitiveComponent.SetCollisionObjectType` _skeletalmesh "ECC_WorldDynamic")
              (`PrimitiveComponent.SetCollisionEnabled` _skeletalmesh "QueryOnly")
              (`PrimitiveComponent.SetCollisionResponseToChannel` _skeletalmesh "ECC_Visibility" "ECR_Block"))
            (:`then_2`
              ;[1 0.3 0] Store all bones Reference Pose Transforms so we don't need to calculate this every time
              (`self.CalculateRefTransforms`))
            (:`then_3`
              ;[0.1 1 0.5 0.5] Create Render Targets
              (bind _returnvalue (`KismetRenderingLibrary.CreateRenderTarget2D` _bloodmasksize _bloodmasksize "RTF_R8"))
              (set `self.BloodMask` _returnvalue)
              (bind _returnvalue_2 (`KismetRenderingLibrary.CreateRenderTarget2D` _bloodmasksize_2 _bloodmasksize_2 "RTF_R8"))
              (set `self.BloodMask_NotDilated` _returnvalue_2)
              (`SceneCaptureComponent.ShowOnlyComponent` _scenecapturecomponent2d (`self.GetMesh`))
              (set `SceneCaptureComponent2D.TextureTarget` (`self.BloodMask_NotDilated`) _scenecapturecomponent2d))
            (:`then_4`
              ;[0.1 1 0.1 0.5] Create render materials
              (bind _returnvalue_3 (`KismetMaterialLibrary.CreateDynamicMaterialInstance` (select `bool` (`self.UseProjectedWound`) :`false` (`self.BloodRenderMaterialAsset`) :`true` (`self.ProjectedWoundRenderMaterialAsset`))))
              (set `self.BloodRenderMaterial` _returnvalue_3)
              (`MaterialInstanceDynamic.SetTextureParameterValue` (`self.BloodRenderMaterial`) "BloodMask" (`self.BloodMask_NotDilated`))
              (if (`self.UseProjectedWound`)
                (`MaterialInstanceDynamic.SetTextureParameterValue` (`self.BloodRenderMaterial`) "WoundTexture" (`self.ProjectedWoundTexture`))))
            (:`then_5`
              (bind _returnvalue_4 (`KismetMaterialLibrary.CreateDynamicMaterialInstance` (`self.BloodDilateMaterialAsset`)))
              (bind _output_get (set `self.DilateMaterial` _returnvalue_4))
              (`MaterialInstanceDynamic.SetScalarParameterValue` _output_get "TextureSize" (`KismetMathLibrary.Conv_IntToDouble` (`self.BloodMaskSize`)))
              (`MaterialInstanceDynamic.SetTextureParameterValue` (`self.DilateMaterial`) "Mask" (`self.BloodMask_NotDilated`)))
            (:`then_6`
              ;[0.1 1 0.1 0.5] Set BloodMask parameter on all materials
              (`self.InitializeMaterials`))
            (:`then_7`
              ;[0.2 0.2 0.2 0.2] Fixes SceneCaptureComponent2D capturing at BeginPlay
              (`KismetSystemLibrary.Delay` 0.1)
              (`KismetRenderingLibrary.ClearRenderTarget2D` (`self.BloodMask`))
              (`KismetRenderingLibrary.ClearRenderTarget2D` (`self.BloodMask_NotDilated`)))))
        (:`Is Not Valid`
          (`KismetSystemLibrary.PrintString` "WoundComponent: Invalid SceneCaptureComponent" false true (struct :`R` 1.0 :`G` 0.144209 :`A` 1.0)))))
    (:`Is Not Valid`
      (`KismetSystemLibrary.PrintString` "WoundComponent: Invalid SkeletalMesh component" false true (struct :`R` 1.0 :`G` 0.144209 :`A` 1.0)))))

(event `TakeHit`
  (params (BoneName :type Name) (WorldSpaceLocation :type "Vector Structure") (HitDirection :type "Vector Structure") (WoundRadius :type "Float (double-precision)" :default 15.0))
  (bind _skeletalmesh (`self.GetMesh`))
  (bind _bloodrendermaterial (`self.BloodRenderMaterial`))
  (if (`self.BloodMaskInitialized`)
    (if (> (`KismetArrayLibrary.Array_Length` (`self.RefPoseLocalBoneTransforms`)) 0)
      (`|ExecutionSequence`
        (:`then_0`
          ;[0 0.2 1 0.2] Send parameters to the render material
          (`MaterialInstanceDynamic.SetVectorParameterValue` _bloodrendermaterial "HitLocation" (`KismetMathLibrary.Conv_VectorToLinearColor` (`self.TransformLocationByRefBoneTransform` BoneName WorldSpaceLocation)))
          (`MaterialInstanceDynamic.SetScalarParameterValue` _bloodrendermaterial "WoundRadius" WoundRadius)
          (if (`self.UseProjectedWound`)
            (`MaterialInstanceDynamic.SetVectorParameterValue` _bloodrendermaterial "HitDirection" (`KismetMathLibrary.Conv_VectorToLinearColor` (`self.TransformDirectionByRefBoneTransform` BoneName HitDirection)))
            (`MaterialInstanceDynamic.SetScalarParameterValue` _bloodrendermaterial "WoundRotation" (`KismetMathLibrary.RandomFloatInRange` 0.0 1.0))))
        (:`then_1`
          ;[0.2 0.2 0.2 0.2] Render the new hit
          (`|ExecutionSequence`
            (:`then_0`
              ;;[0.1 1 0.1 0.5] Set all materials so we can render the hit
              (set `self.TempMaterials` (`MeshComponent.GetMaterials` _skeletalmesh))
              (for (_ _array_index) (`MeshComponent.GetMaterials` _skeletalmesh)
                (`PrimitiveComponent.SetMaterial` _skeletalmesh _array_index (`self.BloodRenderMaterial`))))
            (:`then_1`
              ;;[0.5 0.05 0.05 0.5] Compose the hit into the render target
              (`SceneCaptureComponent2D.CaptureScene` (`self.SceneCaptureComponent2D`)))
            (:`then_2`
              ;;[0.1 1 0.1 0.5] Revert to the original materials
              (for (_ _array_index_2) (`MeshComponent.GetMaterials` _skeletalmesh)
                (`PrimitiveComponent.SetMaterial` _skeletalmesh _array_index_2 (`|GetArrayItem` (`self.TempMaterials`) _array_index_2))))))
        (:`then_2`
          ;[0.5 0.05 0.05 0.5] Dilate the blood mask by one pixel to remove UV seams
          (if (`self.DilateBloodMask`)
            (`KismetRenderingLibrary.DrawMaterialToRenderTarget` (`self.BloodMask`) (`self.DilateMaterial`)))))
      (else
        (`KismetSystemLibrary.PrintString` "WoundComponent could not find any bones in mesh" false true (struct :`R` 1.0 :`G` 0.144209 :`A` 1.0))))
    (else
      (`KismetSystemLibrary.PrintString` "WoundComponent not initialized: At BeginPlay your character needs to call WoundComponent->Initialize" false true (struct :`R` 1.0 :`G` 0.144209 :`A` 1.0)))))

(event `ChangeProjectedWoundTexture`
  (params (Texture2D :type "Texture2D Object Reference"))
  (bind _output_get (set `self.ProjectedWoundTexture` Texture2D))
  (`MaterialInstanceDynamic.SetTextureParameterValue` (`self.BloodRenderMaterial`) "WoundTexture" _output_get))

(fn `CalculateRefTransforms`
  (bind _skeletalmesh (`self.GetMesh`))
  (for _index (range (+ (`SkinnedMeshComponent.GetNumBones` _skeletalmesh) 1))
    (bind _meshlocalspacetransform (`self.GetRefPoseBoneTransform` _skeletalmesh (`SkinnedMeshComponent.GetBoneName` _skeletalmesh _index)))
    (`KismetArrayLibrary.Array_Add` (`self.RefPoseLocalBoneTransforms`) _meshlocalspacetransform)))

(fn `GetMesh`
  (returns (SkeletalMesh :type "SkeletalMeshComponent Object Reference"))
  (return (`self.MeshReference`)))

(fn `GetRefPoseBoneTransform`
  (params (SkeletalMesh :type "SkeletalMeshComponent Object Reference") (BoneName :type Name))
  (returns (MeshLocalSpaceTransform :type "Transform Structure"))
  (locals (BoneTransform :type "Transform Structure"))
  (bind _returnvalue (`SkinnedMeshComponent.GetParentBone` SkeletalMesh BoneName))
  (bind _returnvalue_2 (`KismetMathLibrary.InvertTransform` (`SkinnedMeshComponent.GetDeltaTransformFromRefPose` SkeletalMesh BoneName "None")))
  (if (!= _returnvalue "None")
    (bind _meshlocalspacetransform (`self.GetRefPoseBoneTransform` SkeletalMesh _returnvalue))
    (set `local.BoneTransform` (`KismetMathLibrary.ComposeTransforms` (`KismetMathLibrary.ComposeTransforms` _returnvalue_2 (`SceneComponent.GetSocketTransform` SkeletalMesh BoneName "RTS_ParentBoneSpace")) _meshlocalspacetransform))
    (else
      (set `local.BoneTransform` (`KismetMathLibrary.ComposeTransforms` _returnvalue_2 (`SceneComponent.GetSocketTransform` SkeletalMesh BoneName "RTS_World")))))
  (return (`local.BoneTransform`)))

(fn `InitializeMaterials`
  (locals (Mats :type "Array of MaterialInterface Object Reference"))
  (bind _skeletalmesh (`self.GetMesh`))
  (for (_ _array_index) (`MeshComponent.GetMaterials` _skeletalmesh)
    (bind _returnvalue (`PrimitiveComponent.CreateDynamicMaterialInstance` _skeletalmesh _array_index null "None"))
    (`MaterialInstanceDynamic.SetTextureParameterValue` _returnvalue "BloodMask" (select `bool` (`self.DilateBloodMask`) :`false` (`self.BloodMask_NotDilated`) :`true` (`self.BloodMask`)))))

(fn `TransformDirectionByRefBoneTransform`
  (params (BoneName :type Name) (WorldDirection :type "Vector Structure"))
  (returns (MeshLocalSpaceDirection :type "Vector Structure"))
  (bind _skeletalmesh (`self.GetMesh`))
  (bind _returnvalue (`SkinnedMeshComponent.GetBoneIndex` _skeletalmesh BoneName))
  (if (!= _returnvalue -1)
    (return (`KismetMathLibrary.TransformDirection` (`KismetMathLibrary.ComposeTransforms` (`KismetMathLibrary.InvertTransform` (`SceneComponent.GetSocketTransform` _skeletalmesh BoneName "RTS_Component")) (`|GetArrayItem` (`self.RefPoseLocalBoneTransforms`) _returnvalue)) (`KismetMathLibrary.InverseTransformDirection` (`SceneComponent.K2_GetComponentToWorld` _skeletalmesh) WorldDirection)))
    (else
      (`self.WarningBoneName` BoneName))))

(fn `TransformLocationByRefBoneTransform`
  (params (BoneName :type Name) (WorldLocation :type "Vector Structure"))
  (returns (MeshLocalSpaceLocation :type "Vector Structure"))
  (bind _skeletalmesh (`self.GetMesh`))
  (bind _returnvalue (`SkinnedMeshComponent.GetBoneIndex` _skeletalmesh BoneName))
  (if (!= _returnvalue -1)
    (return (`KismetMathLibrary.TransformLocation` (`KismetMathLibrary.ComposeTransforms` (`KismetMathLibrary.InvertTransform` (`SceneComponent.GetSocketTransform` _skeletalmesh BoneName "RTS_Component")) (`|GetArrayItem` (`self.RefPoseLocalBoneTransforms`) _returnvalue)) (`KismetMathLibrary.InverseTransformLocation` (`SceneComponent.K2_GetComponentToWorld` _skeletalmesh) WorldLocation)))
    (else
      (`self.WarningBoneName` BoneName))))

(fn `WarningBoneName`
  (params (BoneName :type Name))
  (`KismetSystemLibrary.PrintString` (`KismetStringLibrary.Concat_StrStr` "Warning: Wound System Invalid Bone Name : " (`KismetStringLibrary.Conv_NameToString` BoneName)) true true (struct :`R` 1.0 :`G` 0.797118 :`A` 1.0)))